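; Bot car actor that drives itself along a spline path in the level.
; On BeginPlay it finds a SplinePathBP actor and starts a timeline whose play rate is the inverse of TimeToComplete.
; Each update maps the timeline track to a distance along the spline and sets the car's world location and rotation from that point, with scale fixed at half size.
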(event `Move Object`
  (bind _spline (`/Game/Bot_Blueprint/SplinePathBP.Spline` (`self.Spline REF`)))
  (`TimelineComponent.SetPlayRate` (`self.Move Object T`) (/ 1.0 (`self.Time To Complete`)))
  (bind (_direction _move_track) (`Timeline|Move Object T`)
    (:`Update`
      (bind _returnvalue (`KismetMathLibrary.Lerp` 0.0 (`SplineComponent.GetSplineLength` (`/Game/Bot_Blueprint/SplinePathBP.Spline` (`self.Spline REF`))) _move_track))
      (`self.K2_SetActorTransform` (`KismetMathLibrary.MakeTransform` (`SplineComponent.GetLocationAtDistanceAlongSpline` _spline _returnvalue "World") (`SplineComponent.GetRotationAtDistanceAlongSpline` _spline _returnvalue "World") (0.5 0.5 0.5))))))

(event `self.ReceiveBeginPlay`
  (bind _returnvalue (`GameplayStatics.GetActorOfClass` "/Game/Bot_Blueprint/SplinePathBP.SplinePathBP_C"))
  (set `self.Spline REF` _returnvalue)
  (`self.Move Object`))

(fn `UserConstructionScript`)