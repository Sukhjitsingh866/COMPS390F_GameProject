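; BP_StartLine is a start line trigger that starts the race and counts laps for the player's VehicleBlueprint.
; BeginPlay caches the player vehicle and casts its own owner to BP_Checkpoints.
; The first box overlap starts a lap and the race.
; Later overlaps count a lap only when the vehicle's checkpoint text matches a hardcoded "6 / 6", then start the next lap, update laps and unhide the owning checkpoint actor.
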(event `self.ReceiveBeginPlay`
  (bind _asvehicle_blueprint (cast `/Game/VehicleAdvBP/Blueprints/VehicleBlueprint` (`GameplayStatics.GetPlayerPawn` 0)))
  (set `self.As Vehicle Blueprint` _asvehicle_blueprint)
  (set `self.As BP Checkpoint Manager` null)
  (bind _asbp_checkpoints (cast `/Game/rvs_part/BP_Checkpoints` (`self.GetOwner`)))
  (set `self.As BP Checkpoints` _asbp_checkpoints))

(event `self.Box.OnComponentBeginOverlap`
  (params (OverlappedComponent :type "PrimitiveComponent Object Reference") (OtherActor :type "Actor Object Reference") (OtherComp :type "PrimitiveComponent Object Reference") (OtherBodyIndex :type Integer) (bFromSweep :type Boolean) (SweepResult :type "HitResult Structure (by ref)"))
  (bind _as_vehicle_blueprint (`self.As Vehicle Blueprint`))
  (if (`self.DidTheRaceStart`)
    (if (`KismetStringLibrary.EqualEqual_StrStr` (`KismetTextLibrary.Conv_TextToString` (`/Game/VehicleAdvBP/Blueprints/VehicleBlueprint.CheckpointText` (`self.As Vehicle Blueprint`))) "6 / 6")
      (`/Engine/EditorBlueprintResources/StandardMacros.IncrementInt` (`/Game/VehicleAdvBP/Blueprints/VehicleBlueprint.LapsCompleted` _as_vehicle_blueprint)
        (:`  `
          (`/Game/VehicleAdvBP/Blueprints/VehicleBlueprint.StartLap` _as_vehicle_blueprint)
          (`/Game/VehicleAdvBP/Blueprints/VehicleBlueprint.Update Laps` _as_vehicle_blueprint)
          (`self.SetActorHiddenInGame` (`self.As BP Checkpoints`) false))))
    (else
      (`/Game/VehicleAdvBP/Blueprints/VehicleBlueprint.StartLap` _as_vehicle_blueprint)
      (`/Engine/EditorBlueprintResources/StandardMacros.DoOnce` false
        (:`Completed`
          (`/Game/VehicleAdvBP/Blueprints/VehicleBlueprint.Start Race` _as_vehicle_blueprint)
          (set `self.DidTheRaceStart` true))))))

(fn `UserConstructionScript`)