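; Checkpoint manager that tracks how many of its checkpoints the player vehicle has hit in a lap.
; On BeginPlay it binds to each checkpoint's hit event and caches the player's VehicleBlueprint.
; Each hit updates the vehicle's checkpoint progress text.
; Reaching the total starts a looping timer that polls the vehicle's LapComplete flag, then clears it, re-shows and re-enables the checkpoints, and zeroes the count.
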(event `self.ReceiveBeginPlay`
  (bind _checkpoints (`self.Checkpoints`))
  (set `self.CheckpointRequired` (`KismetArrayLibrary.Array_Length` _checkpoints))
  (for _array_element _checkpoints
    (add `/Game/checkpoints_finishline/BP_Checkpoints.CheckpointHit` _array_element (delegate `CheckpointHit`))
    (set `/Game/VehicleAdvBP/Blueprints/VehicleBlueprint.CheckpointText` (`self.CheckpointsToText` (`self.CheckpointRequired`)) (`self.As Vehicle Blueprint_0`))
    (bind _asvehicle_blueprint (cast `/Game/VehicleAdvBP/Blueprints/VehicleBlueprint` (`GameplayStatics.GetPlayerPawn` 0)))
    (set `self.As Vehicle Blueprint_0` _asvehicle_blueprint)))

(event `CheckpointHit`
  (bind _checkpointcount (`self.CheckpointCount`))
  (bind _checkpointrequired (`self.CheckpointRequired`))
  (`/Engine/EditorBlueprintResources/StandardMacros.IncrementInt` _checkpointcount
    (:`  `
      (set `/Game/VehicleAdvBP/Blueprints/VehicleBlueprint.CheckpointText` (`self.CheckpointsToText` _checkpointrequired _checkpointcount) (`self.As Vehicle Blueprint_0`))
      (if (>= _checkpointcount _checkpointrequired)
        (`KismetSystemLibrary.K2_SetTimerDelegate` (delegate `ResetCheckpoints`) 1.0 true)))))

(event `ResetCheckpoints`
  (bind _as_vehicle_blueprint_0 (`self.As Vehicle Blueprint_0`))
  (if (`/Game/VehicleAdvBP/Blueprints/VehicleBlueprint.LapComplete` _as_vehicle_blueprint_0)
    (set `/Game/VehicleAdvBP/Blueprints/VehicleBlueprint.LapComplete` false _as_vehicle_blueprint_0)
    (for _array_element (`self.Checkpoints`)
      (`self.SetActorHiddenInGame` _array_element false)
      (`PrimitiveComponent.SetCollisionEnabled` (`/Game/checkpoints_finishline/BP_Checkpoints.Cube` _array_element) "QueryOnly")
      (bind _output_get (set `self.CheckpointCount` 0))
      (set `/Game/VehicleAdvBP/Blueprints/VehicleBlueprint.CheckpointText` (`self.CheckpointsToText` (`self.CheckpointRequired`) _output_get) (`self.As Vehicle Blueprint_0`)))))

(fn `UserConstructionScript`)